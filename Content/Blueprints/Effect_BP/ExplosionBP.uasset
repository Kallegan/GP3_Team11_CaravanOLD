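; Explosion effect actor that activates a Niagara burst on BeginPlay and damages units or enemies touching its sphere.
; Sphere begin-overlap applies damage by "unit" or "Enemy" tag, but a DoOnce before the tag check limits it to the first overlapping actor.
; Niagara activation plays a placeholder sound once, then destroys the actor after a short delay.
; A disconnected overlapping-actors loop for area damage never runs.
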(event `self.Sphere.OnComponentBeginOverlap`
  (params (OverlappedComponent :type "PrimitiveComponent Object Reference") (OtherActor :type "Actor Object Reference") (OtherComp :type "PrimitiveComponent Object Reference") (OtherBodyIndex :type Integer) (bFromSweep :type Boolean) (SweepResult :type "HitResult Structure (by ref)"))
  (`/Engine/EditorBlueprintResources/StandardMacros.DoOnce` false
    (:`Completed`
      (if (`self.ActorHasTag` OtherActor "unit")
        (`KismetSystemLibrary.PrintString` (`KismetSystemLibrary.GetDisplayName` OtherActor))
        (`GameplayStatics.ApplyDamage` OtherActor 50.0 null self)
        (elif (`self.ActorHasTag` OtherActor "Enemy")
          (`GameplayStatics.ApplyDamage` OtherActor 50.0 null self))))))

(event `self.ReceiveBeginPlay`
  (`ActorComponent.Activate` (`self.Niagara_Explosion`) false))

(event `self.Niagara_Explosion.OnComponentActivated`
  (params (Component :type "ActorComponent Object Reference") (bReset :type Boolean))
  (`/Engine/EditorBlueprintResources/StandardMacros.DoOnce` false
    (:`Completed`
      (`GameplayStatics.PlaySoundAtLocation` "/Game/Audio/PlaceHolder_Explosion_2.PlaceHolder_Explosion_2" (`SceneComponent.K2_GetComponentLocation` (`self.Niagara_Explosion`)) (struct) 0.2 1.0 0.0 null null null null)
      (`KismetSystemLibrary.PrintString` "how many times")
      (`KismetSystemLibrary.Delay` 2.0)
      (`self.K2_DestroyActor`))))

(fn `UserConstructionScript`)