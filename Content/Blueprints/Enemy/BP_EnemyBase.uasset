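; Base enemy Blueprint that senses the player with overlap spheres and passes the results to its AI Blackboard.
; The detection sphere sets CanSeePlayer without ever clearing it here, and writes PlayerREF, which is assigned to itself rather than the overlapping actor.
; The attack-range sphere toggles PlayerIsInRange on begin and end overlap, with debug prints throughout.
; OnDeathBPEvent destroys the actor.
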(event `self.DetectPlayerSphere.OnComponentBeginOverlap`
  (params (OverlappedComponent :type "PrimitiveComponent Object Reference") (OtherActor :type "Actor Object Reference") (OtherComp :type "PrimitiveComponent Object Reference") (OtherBodyIndex :type Integer) (bFromSweep :type Boolean) (SweepResult :type "HitResult Structure (by ref)"))
  (bind _returnvalue (`AIBlueprintHelperLibrary.GetBlackboard` null))
  ;[1 1 1] DetectPlayer
  (if (`self.ActorHasTag` OtherActor "Player")
    (bind _output_get (set `self.PlayerREF` (`self.PlayerREF`)))
    (`BlackboardComponent.SetValueAsObject` _returnvalue "PlayerREF" _output_get)
    (`BlackboardComponent.SetValueAsBool` _returnvalue "CanSeePlayer" true)
    (`KismetSystemLibrary.PrintString` "I See You")))

(event `self.DetectAttackRangeSphere.OnComponentBeginOverlap`
  (params (OverlappedComponent :type "PrimitiveComponent Object Reference") (OtherActor :type "Actor Object Reference") (OtherComp :type "PrimitiveComponent Object Reference") (OtherBodyIndex :type Integer) (bFromSweep :type Boolean) (SweepResult :type "HitResult Structure (by ref)"))
  ;[1 1 1] Check If in attack range
  (if (`self.ActorHasTag` OtherActor "Player")
    (`BlackboardComponent.SetValueAsBool` (`AIBlueprintHelperLibrary.GetBlackboard` null) "PlayerIsInRange" true)
    (`KismetSystemLibrary.PrintString` "I Attack YOu")))

(event `self.OnDeathBPEvent`
  (`self.K2_DestroyActor`))

(event `self.DetectAttackRangeSphere.OnComponentEndOverlap`
  (params (OverlappedComponent :type "PrimitiveComponent Object Reference") (OtherActor :type "Actor Object Reference") (OtherComp :type "PrimitiveComponent Object Reference") (OtherBodyIndex :type Integer))
  ;[1 1 1] Check If in attack range
  (if (`self.ActorHasTag` OtherActor "Player")
    (`BlackboardComponent.SetValueAsBool` (`AIBlueprintHelperLibrary.GetBlackboard` null) "PlayerIsInRange" false)
    (`KismetSystemLibrary.PrintString` "I cant Attack you")))

(fn `UserConstructionScript`)