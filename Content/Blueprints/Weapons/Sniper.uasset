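; Sniper weapon Blueprint that automatically picks and attacks enemies within range.
; Each tick it attacks the current ShootTarget while that reference is valid.
; Without a valid target, it gathers BP_Enemy actors overlapping SphereCollider and selects the one nearest to itself.
; A target is kept until it becomes invalid, with no range recheck.
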(event `self.ReceiveTick`
  (params (DeltaSeconds :type "Float (single-precision)"))
  (`/Engine/EditorBlueprintResources/StandardMacros.IsValid` (`self.ShootTarget`)
    (:`Is Valid`
      (`self.Attack` (`self.ShootTarget`)))
    (:`Is Not Valid`
      (set `self.TargetArray` (`PrimitiveComponent.GetOverlappingActors` (`self.SphereCollider`) "/Game/Blueprints/Enemy/BP_Enemy.BP_Enemy_C"))
      (set `self.ShootTarget` (`.ReturnValue` (`GameplayStatics.FindNearestActor` (`self.K2_GetActorLocation`) (`self.TargetArray`)))))))

(fn `UserConstructionScript`)