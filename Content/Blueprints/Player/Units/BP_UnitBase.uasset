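; BP_UnitBase is a selectable, commandable unit that carries a sniper weapon.
; Move commands halt the AI controller's current movement and issue AIMoveTo to the new location, while selection events toggle a decal.
; The weapon is a separate Sniper actor spawned on BeginPlay and synced to the unit's transform every Tick rather than attached.
; OnDeathBPEvent, fired from C++ at zero HP, destroys both weapon and unit.
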(event `/Game/Blueprints/UI/BPI_UserInterface.UnitMoveCommand`
  (params (Location :type "Vector Structure"))
  (bind _returnvalue (`AIBlueprintHelperLibrary.GetAIController` self))
  ;[1 1 1] Unit move command
  (`Controller.StopMovement` _returnvalue)
  (`AITask_MoveTo.AIMoveTo` _returnvalue Location null))

(event `/Game/Blueprints/UI/BPI_UserInterface.SelectUnits`
  ;[1 1 1] Show / hide decal when unit is selected
  (`SceneComponent.SetVisibility` (`self.UnitSelectedDecal`) true false))

(event `/Game/Blueprints/UI/BPI_UserInterface.DeselectUnits`
  ;[1 1 1] Show / hide decal when unit is selected
  (`SceneComponent.SetVisibility` (`self.UnitSelectedDecal`) false false))

(event `self.OnDeathBPEvent`
  ;[1 1 1] Destroys actor and weapon with c++ fires at 0 hp.
  (`self.K2_DestroyActor` (`self.SniperActor`))
  (`self.K2_DestroyActor`))

(event `self.ReceiveTick`
  (params (DeltaSeconds :type "Float (single-precision)"))
  ;[1 1 1] Updates weapon position and rotation
  (`self.K2_SetActorLocation` (`self.SniperActor`) (`self.K2_GetActorLocation`) false false)
  (`self.K2_SetActorRotation` (`self.SniperActor`) (`self.K2_GetActorRotation`) false))

(event `self.ReceiveBeginPlay`
  ;[1 1 1] Spawns the weapon
  (bind _returnvalue (`|SpawnActorFromClass` "/Game/Blueprints/Weapons/Sniper.Sniper_C" (`KismetMathLibrary.Conv_VectorToTransform` (`self.K2_GetActorLocation`)) "AlwaysSpawn" "OverrideRootScale" (`self.GetOwner`) null))
  (bind _output_get (set `self.SniperActor` _returnvalue))
  (`self.K2_SetActorRotation` _output_get (`self.K2_GetActorRotation`) false))

(fn `GrabSelectedUnits`
  (returns (Units :type "Array of Actor Object Reference"))
  (return))

(fn `UserConstructionScript`)