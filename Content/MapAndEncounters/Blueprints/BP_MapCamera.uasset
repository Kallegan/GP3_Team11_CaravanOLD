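; BP_MapCamera is a map camera actor with edge-scrolling logic that is currently disconnected.
; The MouseX and MouseY events are empty, and the only live behavior is a debug "Hello" print on actor overlap.
; The unused chains compare mouse position to viewport size and apply swept, delta-time-scaled world offsets at ScrollSpeed near screen edges.
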(event `self.ReceiveActorBeginOverlap`
  (params (OtherActor :type "Actor Object Reference"))
  (`KismetSystemLibrary.PrintString` "Hello"))

(event `InputAxisKey|MouseX`
  (params (AxisValue :type "Float (single-precision)"))
  ;[1 1 1] edge scrolling
)

(event `InputAxisKey|MouseY`
  (params (AxisValue :type "Float (single-precision)"))
  ;[1 1 1] edge scrolling
)

(fn `UserConstructionScript`)