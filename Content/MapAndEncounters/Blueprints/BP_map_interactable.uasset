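; Map interactable with three clickable nodes, each a box and cylinder pair that opens its own hard-wired desert level.
; Cursor hover over a box lifts its cylinder with physics off; leaving re-enables physics to drop it unless a node was clicked.
; Clicking fades the camera out while a timeline spins the cylinder, then loads the level after a short delay.
; An unconnected leftover would launch the caravan toward the middle cylinder.
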(event `self.Box0.OnClicked`
  (params (TouchedComponent :type "PrimitiveComponent Object Reference") (ButtonPressed :type "Key Structure"))
  ;[1 1 1] choose levels to open here for now
  (set `self.bNodeClicked?` true)
  (`PlayerCameraManager.StartCameraFade` :`self` (`GameplayStatics.GetPlayerCameraManager` 0) :`ToAlpha` 1.0 :`Duration` 1.0 :`bHoldWhenFinished` true)
  (`Timeline|Timeline_0` :!via `PlayFromStart`
    (:`Update`
      (`SceneComponent.K2_AddWorldRotation` (`self.Cylinder0`) (struct :`Pitch` 10.0) false false)
      (`KismetSystemLibrary.Delay` 1.0)
      (`GameplayStatics.OpenLevelBySoftObjectPtr` "/Game/Levels/Salt_Plains_Levels/SaltPlanes_1.SaltPlanes_1"))))

(event `self.Box1.OnClicked`
  (params (TouchedComponent :type "PrimitiveComponent Object Reference") (ButtonPressed :type "Key Structure"))
  ;[1 1 1] choose levels to open here for now
  (set `self.bNodeClicked?` true)
  (`PlayerCameraManager.StartCameraFade` :`self` (`GameplayStatics.GetPlayerCameraManager` 0) :`ToAlpha` 1.0 :`Duration` 1.0 :`bHoldWhenFinished` true)
  (`Timeline|Timeline_1` :!via `PlayFromStart`
    (:`Update`
      (`SceneComponent.K2_AddWorldRotation` (`self.Cylinder1`) (struct :`Pitch` 10.0) false false)
      (`KismetSystemLibrary.Delay` 1.0)
      (`GameplayStatics.OpenLevelBySoftObjectPtr` "/Game/Levels/Sand_Dunes_Levels/SandDunes2.SandDunes2"))))

(event `self.Box2.OnClicked`
  (params (TouchedComponent :type "PrimitiveComponent Object Reference") (ButtonPressed :type "Key Structure"))
  ;[1 1 1] choose levels to open here for now
  (set `self.bNodeClicked?` true)
  (`PlayerCameraManager.StartCameraFade` :`self` (`GameplayStatics.GetPlayerCameraManager` 0) :`ToAlpha` 1.0 :`Duration` 1.0 :`bHoldWhenFinished` true)
  (`Timeline|Timeline_2` :!via `PlayFromStart`
    (:`Update`
      (`SceneComponent.K2_AddWorldRotation` (`self.Cylinder2`) (struct :`Pitch` 10.0) false false)
      (`KismetSystemLibrary.Delay` 1.0)
      (`GameplayStatics.OpenLevelBySoftObjectPtr` "/Game/Levels/Sand_Dunes_Levels/SandDunes_1NoBlockout.SandDunes_1NoBlockout"))))

(event `self.Box0.OnBeginCursorOver`
  (params (TouchedComponent :type "PrimitiveComponent Object Reference"))
  (bind _cylinder0 (`self.Cylinder0`))
  (if (not (`self.bCylinder0 in air?`))
    (`PrimitiveComponent.SetSimulatePhysics` _cylinder0 false)
    (`SceneComponent.SetMobility` _cylinder0 "Movable")
    (`SceneComponent.K2_AddWorldOffset` _cylinder0 (0.0 0.0 5.0) false false)
    (set `self.bCylinder0 in air?` true)
    (`KismetSystemLibrary.Delay` 0.5)))

(event `self.Box0.OnEndCursorOver`
  (params (TouchedComponent :type "PrimitiveComponent Object Reference"))
  (if (`self.bNodeClicked?`)
    _
    (elif (`self.bCylinder0 in air?`)
      (`PrimitiveComponent.SetSimulatePhysics` (`self.Cylinder0`) true)
      (`KismetSystemLibrary.Delay` 0.2)
      (set `self.bCylinder0 in air?` false))))

(event `self.Box1.OnBeginCursorOver`
  (params (TouchedComponent :type "PrimitiveComponent Object Reference"))
  (bind _cylinder1 (`self.Cylinder1`))
  (if (not (`self.bCylinder1 in air?`))
    (`PrimitiveComponent.SetSimulatePhysics` _cylinder1 false)
    (`SceneComponent.SetMobility` _cylinder1 "Movable")
    (`SceneComponent.K2_AddWorldOffset` _cylinder1 (0.0 0.0 5.0) false false)
    (set `self.bCylinder1 in air?` true)
    (`KismetSystemLibrary.Delay` 0.5)))

(event `self.Box1.OnEndCursorOver`
  (params (TouchedComponent :type "PrimitiveComponent Object Reference"))
  (if (`self.bNodeClicked?`)
    _
    (elif (`self.bCylinder1 in air?`)
      (`PrimitiveComponent.SetSimulatePhysics` (`self.Cylinder1`) true)
      (`KismetSystemLibrary.Delay` 0.2)
      (set `self.bCylinder1 in air?` false))))

(event `self.Box2.OnBeginCursorOver`
  (params (TouchedComponent :type "PrimitiveComponent Object Reference"))
  (bind _cylinder2 (`self.Cylinder2`))
  (if (not (`self.bCylinder2 in air?`))
    (`PrimitiveComponent.SetSimulatePhysics` _cylinder2 false)
    (`SceneComponent.SetMobility` _cylinder2 "Movable")
    (`SceneComponent.K2_AddWorldOffset` _cylinder2 (0.0 0.0 5.0) false false)
    (set `self.bCylinder2 in air?` true)))

(event `self.Box2.OnEndCursorOver`
  (params (TouchedComponent :type "PrimitiveComponent Object Reference"))
  (if (`self.bNodeClicked?`)
    _
    (elif (`self.bCylinder2 in air?`)
      (`PrimitiveComponent.SetSimulatePhysics` (`self.Cylinder2`) true)
      (`KismetSystemLibrary.Delay` 0.2)
      (set `self.bCylinder2 in air?` false))))

(fn `UserConstructionScript`)